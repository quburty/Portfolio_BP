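; Base weapon Blueprint with empty Attack, EndAttack and AttackRelease functions and shared damage logic.
; Wrappers read and write the owner's state, combat, movement and health through interface messages, though SetCanMove and SetHealth check BP_IWeapon rather than BP_ICharacter.
; CanAttack gates on combat type and state.
; SendDamage hits other Characters using direct or component-calculated power, boosts BP_Melee air attacks, spawns hit effects and builds BP_Player rage.
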(fn ConstructionScript)

(fn GetState
  (bind _returnvalue (Components|GetOwner))
  (if (Utilities|DoesObjectImplementInterface _returnvalue "/Game/Interfaces/BP_ICharacter.BP_ICharacter_C")
    (bind _state (Class|BPICharacter|GetState(Message) _returnvalue))
    (return _state)))

(fn SetState
  (params (State :type EStateType%20Enum :default "NewEnumerator0"))
  (bind _returnvalue (Components|GetOwner))
  (if (Utilities|DoesObjectImplementInterface _returnvalue "/Game/Interfaces/BP_ICharacter.BP_ICharacter_C")
    (Class|BPICharacter|SetState(Message) _returnvalue State)))

(fn GetCombat
  (bind _returnvalue (Components|GetOwner))
  (if (Utilities|DoesObjectImplementInterface _returnvalue "/Game/Interfaces/BP_ICharacter.BP_ICharacter_C")
    (bind _combattype (Class|BPICharacter|GetCombat(Message) _returnvalue))
    (return _combattype)))

(fn SetCombat
  (params (Combat :type ECombatType%20Enum :default "NewEnumerator0"))
  (bind _returnvalue (Components|GetOwner))
  (if (Utilities|DoesObjectImplementInterface _returnvalue "/Game/Interfaces/BP_ICharacter.BP_ICharacter_C")
    (Class|BPICharacter|SetCombat(Message) _returnvalue Combat)))

(fn CanAttack
  (return (and (Utilities|Enum|Equal(Enum) (CallFunction|GetCombat) (Variables|UserSettings|GetCombatType)) (Utilities|Enum|Equal(Enum) (CallFunction|GetState) "NewEnumerator0"))))

(fn Attack)

(fn EndAttack)

(fn SendDamage
  (params (OtherActor :type Actor%20Object%20Reference) (ApplyPowerDirect :type Boolean) (Power :type Float%20%28single-precision%29))
  (if (!= OtherActor (Components|GetOwner))
    (bind _ascharacter (Utilities|Casting|CastToCharacter OtherActor)
      (:then
        (Utilities|FlowControl|Sequence
          (:then_0
            (if ApplyPowerDirect
              (LocalVariables|SetPowerFinal Power)
              (else
                (LocalVariables|SetPowerFinal (Default|GetAttack (Variables|Default|GetWeaponDamageComponent) (Variables|Default|GetPowerTypeDetail) (Actor|GetComponentbyClass (Components|GetOwner) "/Game/Components/Status/StatusComponent.StatusComponent_C") (Actor|GetComponentbyClass OtherActor "/Game/Components/Status/StatusComponent.StatusComponent_C"))))))
          (:then_1
            (bind _asbp_melee (Utilities|Casting|CastToBP_Melee self))
            (if (Variables|/Game/Weapons/Melees/BP_Melee.BP_Melee_C|GetAirAttack _asbp_melee)
              (LocalVariables|SetPowerFinal (* (LocalVariables|GetPowerFinal) 1.5))))
          (:then_2
            (if (> (LocalVariables|GetPowerFinal) 0.0)
              (bind _returnvalue (Game|Damage|ApplyDamage _ascharacter (LocalVariables|GetPowerFinal) (Game|GetInstigatorController (Components|GetOwner)) self))
              (Utilities|FlowControl|Sequence
                (:then_0
                  (bind _hiteffect (Variables|UserSettings|GetHitEffect)
                    (:then
                      (Effects|SpawnEmitteratLocation _hiteffect (Transformation|GetActorLocation _ascharacter) "0, 0, 0" (Variables|UserSettings|GetHitEffectScale)))
                    (:else)))
                (:then_1
                  (if (> _returnvalue 0.0)
                    (bind _asbp_player (Utilities|Casting|CastToBP_Player (Components|GetOwner)))
                    (Default|IncreaseRage _asbp_player (Variables|Default|GetRageIncreament))))
                (:then_2
                  (return true)))
              (else
                (Development|PrintString "Warning: Damage is 0!"))))))
      (:CastFailed
        (return false)))
    (else
      (return false))))

(fn GetCanMove
  (bind _returnvalue (Components|GetOwner))
  (if (Utilities|DoesObjectImplementInterface _returnvalue "/Game/Interfaces/BP_ICharacter.BP_ICharacter_C")
    (bind _canmove (Class|BPICharacter|GetCanMove(Message) _returnvalue))
    (return _canmove)))

(fn SetCanMove
  (params (CanMove :type Boolean))
  (bind _returnvalue (Components|GetOwner))
  (if (Utilities|DoesObjectImplementInterface _returnvalue "/Game/Interfaces/BP_IWeapon.BP_IWeapon_C")
    (Class|BPICharacter|SetCanMove(Message) _returnvalue CanMove)))

(fn GetHealth
  (bind _returnvalue (Components|GetOwner))
  (if (Utilities|DoesObjectImplementInterface _returnvalue "/Game/Interfaces/BP_ICharacter.BP_ICharacter_C")
    (bind _health (Class|BPICharacter|GetHealth(Message) _returnvalue))
    (return _health)))

(fn SetHealth
  (params (Health :type Float%20%28single-precision%29))
  (bind _returnvalue (Components|GetOwner))
  (if (Utilities|DoesObjectImplementInterface _returnvalue "/Game/Interfaces/BP_IWeapon.BP_IWeapon_C")
    (Class|BPICharacter|SetHealth(Message) _returnvalue Health)))

(fn AttackRelease)