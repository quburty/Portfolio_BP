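; BP_Melee is a melee weapon Blueprint providing combo attacks, air attacks and a cooldown-gated skill.
; Attack starts a montage through owner interface messages or buffers the next combo step, which PlayNextCombo consumes unless a weapon switch is pending.
; Air attacks zero the owner's velocity and gravity until EndAttack restores gravity and resets the combo.
; SendDamage records hit Characters to prevent repeat damage until OffCollision clears the list.
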(event Custom|On%20Collision
  (params (PowerType :type EWeaponPowerType_Detail%20Enum :default "NewEnumerator14"))
  (Variables|Default|SetPowerTypeDetail PowerType))

(event Custom|Off%20Collision
  (Utilities|Array|Clear (Variables|Default|GetHitted))
  (Variables|Default|SetPowerTypeDetail "NewEnumerator14"))

(event EventTick
  (params (DeltaSeconds :type Float%20%28single-precision%29))
  (|CallParentFunction DeltaSeconds)
  (if (> (Variables|Default|GetSkillCoolTimeLeft) 0.0)
    (Variables|Default|SetSkillCoolTimeLeft (- (Variables|Default|GetSkillCoolTimeLeft) DeltaSeconds))))

(event EventBeginPlay
  (|CallParentFunction))

(fn ConstructionScript
  (|CallParentFunction))

(fn PlayComboMontage
  (Class|BPIWeapon|WeaponPlayMeleeMontage(Message) (Components|GetOwner) (Variables|Default|GetCombatType) (Variables|Default|GetMeleeCount)))

(fn SendDamage
  (params (OtherActor :type Actor%20Object%20Reference) (ApplyPowerDirect :type Boolean) (Power :type Float%20%28single-precision%29))
  (bind _array_element (Utilities|Array|ForEachLoopwithBreak (Variables|Default|GetHitted) :!label _label)
    (:LoopBody
      (if (== _array_element OtherActor)
        (LocalVariables|SetFind true)
        (goto _label Break)))
    (:Completed
      (if (not (LocalVariables|GetFind))
        (bind _ascharacter (Utilities|Casting|CastToCharacter OtherActor))
        (Utilities|Array|Add (Variables|Default|GetHitted) _ascharacter)
        (bind _result (|CallParentFunction OtherActor false Power))
        (return _result)))))

(fn CanAttack
  (bind _state (CallFunction|GetState))
  (return (and (Utilities|Enum|Equal(Enum) (CallFunction|GetCombat) (Variables|Default|GetCombatType)) (or (Utilities|Enum|Equal(Enum) _state "NewEnumerator0") (Utilities|Enum|Equal(Enum) _state "NewEnumerator10")))))

(fn Skill
  (bind _returnvalue (Components|GetOwner))
  (if (and (CallFunction|CanAttack) (CallFunction|IsCanUseSkill))
    (Variables|Default|SetSkillCoolTimeLeft (Variables|Default|GetSkillCoolTimeMax))
    (Class|BPICharacter|SetState(Message) _returnvalue "NewEnumerator1")
    (Class|BPIWeapon|WeaponPlaySkillMontage(Message) _returnvalue (Variables|Default|GetCombatType))))

(fn SkillEffect)

(fn IsCanUseSkill
  (return (< (Variables|Default|GetSkillCoolTimeLeft) 1e-05)))

(fn AttachtoSocket
  (params (Component :type Scene%20Component%20Object%20Reference) (SocketName :type Name))
  (bind _ascharacter (Utilities|Casting|CastToCharacter (Components|GetOwner)))
  (bind _returnvalue (Transformation|AttachComponentToComponent Component (Variables|/Script/Engine.Character|GetMesh _ascharacter) SocketName "KeepRelative" "KeepRelative" "KeepRelative" true))
  (return _returnvalue))

(event Custom|SetOwnerFloatAttack
  (params (Float :type Boolean))
  (bind _returnvalue (Components|GetOwner))
  (bind _returnvalue_2 (Actor|GetComponentbyClass _returnvalue "/Script/Engine.CharacterMovementComponent"))
  (bind _asbp_player (Utilities|Casting|CastToBP_Player _returnvalue))
  (Default|SetRotationFree _asbp_player Float)
  (if Float
    (Variables|/Script/Engine.CharacterMovementComponent|SetGravityScale _returnvalue_2 0.0)
    (Variables|/Script/Engine.MovementComponent|SetVelocity _returnvalue_2 (Math|Vector|MakeVector 0.0 0.0 0.0))
    (else
      (Variables|/Script/Engine.CharacterMovementComponent|SetGravityScale _returnvalue_2 1.0))))

(event EventAttack
  (|CallParentFunction)
  (if (Variables|Default|GetEnableNextCombo)
    (Math|Integer|IncrementInt (Variables|Default|GetMeleeCount)
      (:%20%20
        (Variables|Default|SetExistNextCombo true)
        (Variables|Default|SetEnableNextCombo false)))
    (elif (CallFunction|CanAttack)
      (bind _state (Class|BPICharacter|GetState(Message) (Components|GetOwner)))
      (if (or (Utilities|Enum|Equal(Enum) _state "NewEnumerator10") (Utilities|Enum|Equal(Enum) _state "NewEnumerator11"))
        (CallFunction|SetState "NewEnumerator11")
        (CallFunction|SetOwnerFloatAttack true)
        (Variables|Default|SetAirAttack true)
        (else
          (CallFunction|SetState "NewEnumerator1")))
      (CallFunction|PlayComboMontage))))

(event Custom|PlayNextCombo
  (if (Variables|Default|GetExistSwitching)
    (Variables|Default|SetExistSwitching false)
    (Variables|Default|SetExistNextCombo false)
    (bind _asbp_player (Utilities|Casting|CastToBP_Player (Components|GetOwner)))
    (Default|SwitchWeaponAtk _asbp_player)
    (elif (Variables|Default|GetExistNextCombo)
      (CallFunction|PlayCombo))))

(event Custom|PlayCombo
  (CallFunction|PlayComboMontage)
  (Variables|Default|SetExistNextCombo false))

(event EventEndAttack
  (if (Variables|Default|GetAirAttack)
    (CallFunction|SetState "NewEnumerator10")
    (CallFunction|SetOwnerFloatAttack false))
  (CallFunction|SetState "NewEnumerator0")
  (CallFunction|SetCanMove true)
  (Variables|Default|SetExistNextCombo false)
  (Variables|Default|SetMeleeCount 0)
  (Variables|Default|SetLastCombo false)
  (Variables|Default|SetAirAttack false))