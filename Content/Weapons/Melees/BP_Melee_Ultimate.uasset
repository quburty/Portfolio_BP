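; BP_Melee_Ultimate is a melee weapon Blueprint, likely for an ultimate attack, that damages actors overlapping its capsule.
; On BeginPlay it disables collision and hides the root with all child components.
; OnCollision and OffCollision extend the parent's events by enabling or disabling the capsule's collision.
; Each capsule overlap passes the other actor to SendDamage, without applying direct power.
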(event OnComponentBeginOverlap(Capsule)
  (params (OverlappedComponent :type Primitive%20Component%20Object%20Reference) (OtherActor :type Actor%20Object%20Reference) (OtherComp :type Primitive%20Component%20Object%20Reference) (OtherBodyIndex :type Integer) (bFromSweep :type Boolean) (SweepResult :type Hit%20Result%20Structure%20%28by%20ref%29))
  (CallFunction|SendDamage OtherActor false 0.0))

(event EventOnCollision
  (params (PowerType :type EWeaponPowerType_Detail%20Enum :default "NewEnumerator14"))
  (|CallParentFunction PowerType)
  (Collision|SetCollisionEnabled (Variables|Default|GetCapsule) "QueryAndPhysics"))

(event EventOffCollision
  (|CallParentFunction)
  (Collision|SetCollisionEnabled (Variables|Default|GetCapsule) "NoCollision"))

(event EventBeginPlay
  (CallFunction|OffCollision)
  (Rendering|SetVisibility (Variables|Default|GetDefaultSceneRoot) false true)
  (|CallParentFunction))

(fn ConstructionScript)