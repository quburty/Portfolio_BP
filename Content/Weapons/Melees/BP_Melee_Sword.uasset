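; BP_Melee_Sword is a melee weapon that deals damage through a capsule overlap and adds a dash skill.
; Its collision starts disabled and is toggled by OnCollision and OffCollision, which extend the parent's handlers; overlaps send fixed-power damage.
; SkillEffect alternates between launching the owning Character forward and zeroing its velocity, briefly enabling movement for each change before locking it again.
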(event OnComponentBeginOverlap(Capsule)
  (params (OverlappedComponent :type Primitive%20Component%20Object%20Reference) (OtherActor :type Actor%20Object%20Reference) (OtherComp :type Primitive%20Component%20Object%20Reference) (OtherBodyIndex :type Integer) (bFromSweep :type Boolean) (SweepResult :type Hit%20Result%20Structure%20%28by%20ref%29))
  (CallFunction|SendDamage OtherActor false 2e+01))

(event EventOnCollision
  (params (PowerType :type EWeaponPowerType_Detail%20Enum :default "NewEnumerator14"))
  (|CallParentFunction PowerType)
  (Collision|SetCollisionEnabled (Variables|Default|GetCapsule) "QueryAndPhysics"))

(event EventOffCollision
  (|CallParentFunction)
  (Collision|SetCollisionEnabled (Variables|Default|GetCapsule) "NoCollision"))

(event EventBeginPlay
  (CallFunction|OffCollision)
  (|CallParentFunction))

(fn ConstructionScript)

(event EventSkillEffect
  (|CallParentFunction)
  (bind _ascharacter (Utilities|Casting|CastToCharacter (Components|GetOwner)))
  (if (Variables|Default|GetIsSkillEffectSecond)
    (CallFunction|SetCanMove true)
    (Variables|/Script/Engine.MovementComponent|SetVelocity (Variables|/Script/Engine.Character|GetCharacterMovement _ascharacter) "0, 0, 0")
    (CallFunction|SetCanMove false)
    (Variables|Default|SetIsSkillEffectSecond false)
    (else
      (CallFunction|SetCanMove true)
      (Character|LaunchCharacter _ascharacter (* (Transformation|GetActorForwardVector _ascharacter) 5e+03) false false)
      (CallFunction|SetCanMove false)
      (Variables|Default|SetIsSkillEffectSecond true))))