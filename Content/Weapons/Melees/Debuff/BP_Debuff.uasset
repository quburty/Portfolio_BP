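; BP_Debuff is a short-lived damage-over-time debuff actor that hurts its owner.
; BeginPlay sets a three-second lifespan, so the actor destroys itself.
; Tick accumulates delta time and, each time it passes one second, resets it and applies fixed damage to the owner.
; Damage is credited to the instigator's controller, with the debuff itself as the causer.
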(event EventBeginPlay
  (Actor|SetLifeSpan 3.0))

(event Collision|EventActorBeginOverlap
  (params (OtherActor :type Actor%20Object%20Reference)))

(event EventTick
  (params (DeltaSeconds :type Float%20%28single-precision%29))
  (bind _output_get (Variables|Default|SetTime (+ DeltaSeconds (Variables|Default|GetTime))))
  (if (> _output_get 1.0)
    (Variables|Default|SetTime 0.0)
    (Game|Damage|ApplyDamage (Components|GetOwner) 5.0 (Game|GetInstigatorController (Game|GetInstigator)) self)))

(fn ConstructionScript)