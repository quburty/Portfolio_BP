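; Anim notify state that marks the combo window in melee attack animations, shown as "EnableNextCombo".
; On begin and end it gets the owner's current weapon through the BP_ICharacter interface and casts it to BP_Melee.
; It sets that weapon's EnableNextCombo flag true for the notify's duration and false when it ends.
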(fn GetNotifyName
  (return "EnableNextCombo"))

(fn ReceivedNotifyBegin
  (params (MeshComp :type Skeletal%20Mesh%20Component%20Object%20Reference) (Animation :type Anim%20Sequence%20Base%20Object%20Reference) (TotalDuration :type Float%20%28single-precision%29))
  (bind _returnvalue (Components|GetOwner MeshComp))
  (if (Utilities|DoesObjectImplementInterface _returnvalue "/Game/Interfaces/BP_ICharacter.BP_ICharacter_C")
    (bind _currentweapon (Class|BPIWeapon|GetCurrentWeapon(Message) _returnvalue))
    (bind _asbp_melee (Utilities|Casting|CastToBP_Melee _currentweapon))
    (Variables|/Game/Weapons/Melees/BP_Melee.BP_Melee_C|SetEnableNextCombo _asbp_melee true)
    (return false)))

(fn ReceivedNotifyEnd
  (params (MeshComp :type Skeletal%20Mesh%20Component%20Object%20Reference) (Animation :type Anim%20Sequence%20Base%20Object%20Reference))
  (bind _returnvalue (Components|GetOwner MeshComp))
  (if (Utilities|DoesObjectImplementInterface _returnvalue "/Game/Interfaces/BP_ICharacter.BP_ICharacter_C")
    (bind _currentweapon (Class|BPIWeapon|GetCurrentWeapon(Message) _returnvalue))
    (bind _asbp_melee (Utilities|Casting|CastToBP_Melee _currentweapon))
    (Variables|/Game/Weapons/Melees/BP_Melee.BP_Melee_C|SetEnableNextCombo _asbp_melee false)
    (return false)))