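; Anim notify state named "Collision" that opens and closes a melee weapon's hit collision window during attack animations.
; On begin, it gets the mesh owner's current weapon, casts it to BP_Melee and calls OnCollision with the notify's PowerTypeDetail.
; On end, it fetches the weapon the same way and calls OffCollision, doing nothing if the weapon is not melee.
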(fn GetNotifyName
  (return "Collision"))

(fn ReceivedNotifyBegin
  (params (MeshComp :type Skeletal%20Mesh%20Component%20Object%20Reference) (Animation :type Anim%20Sequence%20Base%20Object%20Reference) (TotalDuration :type Float%20%28single-precision%29))
  (bind _currentweapon (Class|BPIWeapon|GetCurrentWeapon(Message) (Components|GetOwner MeshComp)))
  (bind _asbp_melee (Utilities|Casting|CastToBP_Melee _currentweapon))
  (Default|OnCollision _asbp_melee (Variables|Default|GetPowerTypeDetail))
  (return false))

(fn ReceivedNotifyEnd
  (params (MeshComp :type Skeletal%20Mesh%20Component%20Object%20Reference) (Animation :type Anim%20Sequence%20Base%20Object%20Reference))
  (bind _currentweapon (Class|BPIWeapon|GetCurrentWeapon(Message) (Components|GetOwner MeshComp)))
  (bind _asbp_melee (Utilities|Casting|CastToBP_Melee _currentweapon))
  (Default|OffCollision _asbp_melee)
  (return false))