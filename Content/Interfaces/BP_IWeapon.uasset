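; BP_IWeapon is a Blueprint interface for a weapon system, declaring functions only, with no logic.
; It covers changing and querying the current weapon, hit notification, and equip, sheathe, grab and ungrab actions, several of which take a Combat argument.
; Montage functions cover draw, sheath, melee and skill animations, with melee selected by combat type and melee count and skill by combat type.
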(fn WeaponChange
  (params (New%20Weapon :type BP%20Weapon%20Object%20Reference))
  (return 0))

(fn WeaponHitted
  (return false))

(fn WeaponSheathed
  (return false))

(fn WeaponEquipped
  (params (Combat :type ECombatType%20Enum :default "NewEnumerator0"))
  (return false))

(fn WeaponGrab
  (params (Combat :type ECombatType%20Enum :default "NewEnumerator0"))
  (return false))

(fn WeaponUngrab
  (params (Combat :type ECombatType%20Enum :default "NewEnumerator0"))
  (return false))

(fn WeaponPlayMeleeMontage
  (params (CombatType :type ECombatType%20Enum :default "NewEnumerator0") (MeleeCount :type Integer))
  (return false))

(fn WeaponPlaySkillMontage
  (params (CombatType :type ECombatType%20Enum :default "NewEnumerator0"))
  (return false))

(fn GetCurrentWeapon
  (return 0))

(fn WeaponPlayDrawMontage
  (return false))

(fn WeaponPlaySheathMontage
  (return false))