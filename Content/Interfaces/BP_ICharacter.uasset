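; BP_ICharacter is a Blueprint interface that exposes a character's state, combat type, movement permission and health to other objects.
; It declares getter and setter pairs for the state and combat enums, the can-move flag and health, plus an IsAlive query.
; The setters also return a value of the matching type, and every function body holds only a default return, leaving the logic to implementers.
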(fn GetState
  (return "NewEnumerator0"))

(fn SetState
  (params (StateType :type EStateType%20Enum :default "NewEnumerator0"))
  (return "NewEnumerator0"))

(fn GetCombat
  (return "NewEnumerator0"))

(fn SetCombat
  (params (CombatType :type ECombatType%20Enum :default "NewEnumerator0"))
  (return "NewEnumerator0"))

(fn GetCanMove
  (return false))

(fn SetCanMove
  (params (CanMove :type Boolean))
  (return false))

(fn GetHealth
  (return 0.0))

(fn SetHealth
  (params (Health :type Float%20%28single-precision%29))
  (return 0.0))

(fn IsAlive
  (return false))