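; Sword-wielding enemy AI character that spawns a greatsword on BeginPlay and moves it between holster and hand sockets.
; Weapon functions handle grab, ungrab, equip and sheathe, updating state and combat type enums.
; Melee montages and movement permission come from a map keyed by combat type, while back-step plays its own montage.
; A dot product against the damage causer's position multiplies damage from behind tenfold before passing it to the parent.
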(event EventBeginPlay
  (|CallParentFunction)
  (bind _returnvalue (Game|SpawnActorfromClass "/Game/Weapons/Melees/BP_Melee_GreatSword_Enemy.BP_Melee_GreatSword_Enemy_C" (Math|Transform|MakeTransform "0, 0, 0") "Undefined" self 0))
  (bind _output_get (Variables|Default|SetWeapon _returnvalue))
  (Transformation|AttachComponentToComponent _output_get (Variables|Character|GetMesh) "Holster_GreatSword" "KeepRelative" "KeepRelative" "KeepRelative" true))

(event EventEquipped
  (Variables|Default|SetStateType "NewEnumerator0")
  (Variables|Default|SetCombatType "NewEnumerator9"))

(event EventSheathed
  (Variables|Default|SetStateType "NewEnumerator0")
  (Variables|Default|SetCombatType "NewEnumerator0"))

(event EventGrab
  (Transformation|AttachComponentToComponent (Variables|Default|GetWeapon) (Variables|Character|GetMesh) "Hand_Weapon" "KeepRelative" "KeepRelative" "KeepRelative" true))

(event EventUngrab
  (Transformation|AttachComponentToComponent (Variables|Default|GetWeapon) (Variables|Character|GetMesh) "Holster_GreatSword" "KeepRelative" "KeepRelative" "KeepRelative" true))

(event Game|Damage|EventAnyDamage
  (params (Damage :type Float%20%28single-precision%29) (DamageType :type Damage%20Type%20Object%20Reference) (InstigatedBy :type Controller%20Object%20Reference) (DamageCauser :type Actor%20Object%20Reference))
  (if (< (Math|Vector|DotProduct (- (Transformation|GetActorLocation DamageCauser) (Transformation|GetActorLocation)) (Transformation|GetActorForwardVector)) 0.0)
    (|CallParentFunction (* Damage 1e+01) DamageType InstigatedBy DamageCauser)
    (else
      (|CallParentFunction Damage DamageType InstigatedBy DamageCauser))))

(event EventBackStep
  (|CallParentFunction)
  (Variables|Default|SetStateType "NewEnumerator3")
  (Animation|PlayAnimMontage "/Game/Character/Paladin_J/Montages/Paladin_J_BackStep_Montage.Paladin_J_BackStep_Montage" 1.0 "None"))

(fn ConstructionScript
  (|CallParentFunction))

(fn WeaponPlayMeleeMontage
  (params (CombatType :type ECombatType%20Enum :default "NewEnumerator0") (MeleeCount :type Integer))
  (bind _meleemontages (Variables|Default|GetMeleeMontages))
  (bind (_value _returnvalue) (Utilities|Map|Find _meleemontages (Variables|Default|GetCombatType)))
  (bind (_montage _playratio _startsection _canmove) (Utilities|Struct|BreakFMontageData _value))
  (if _returnvalue
    (Animation|PlayAnimMontage _montage _playratio _startsection)
    (CallFunction|SetCanMove _canmove)
    (return true)
    (else
      (return false))))

(fn WeaponGrab
  (params (Combat :type ECombatType%20Enum :default "NewEnumerator0"))
  (CallFunction|Grab)
  (return true))

(fn WeaponUngrab
  (params (Combat :type ECombatType%20Enum :default "NewEnumerator0"))
  (Transformation|AttachComponentToComponent (Variables|Default|GetWeapon) (Variables|Character|GetMesh) "Holster_GreatSword" "KeepRelative" "KeepRelative" "KeepRelative" true)
  (Variables|Default|SetCombatType "NewEnumerator0")
  (return true))

(fn WeaponEquipped
  (params (Combat :type ECombatType%20Enum :default "NewEnumerator0"))
  (|CallParentFunction Combat)
  (CallFunction|Equipped)
  (return true))

(fn WeaponSheathed
  (|CallParentFunction)
  (CallFunction|Sheathed)
  (return true))