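; BP_Enemy is the base enemy character, with health, hit reactions, death and a weapon interface mostly stubbed except melee montages.
; AnyDamage subtracts non-self damage from health, briefly shows the health bar, and triggers montage, damage number, sound and blood effect.
; Hit stop uses global time dilation, stronger and shorter except during the death wait.
; Death stops AI logic, disables capsule collision and destroys the actor near the death montage's end.
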(fn ConstructionScript)

(fn Killed)

(event Custom|UpdateHealthBarEvent
  (bind _status (Variables|Default|GetStatus))
  (Rendering|SetVisibility (Variables|Default|GetHealthBar) true false)
  (Utilities|Time|SetTimerbyEvent (delegate Custom|HideHealthBar) 5.0)
  (bind _aswb_health_bar (Utilities|Casting|CastToWB_HealthBar (UserInterface|GetUserWidgetObject (Variables|Default|GetHealthBar))))
  (Default|UpdateHealthBar _aswb_health_bar (Variables|/Game/Components/Status/StatusComponent.StatusComponent_C|GetHealth _status) (Variables|/Game/Components/Status/StatusComponent.StatusComponent_C|GetMaxHealth _status)))

(event Custom|HideHealthBar
  (Rendering|SetVisibility (Variables|Default|GetHealthBar) false false))

(event EventBeginPlay
  (bind _returnvalue (Rendering|Material|CreateDynamicMaterialInstance (Rendering|Material|GetMaterial (Variables|Character|GetMesh) 1) "None" :!class /Script/Engine.KismetMaterialLibrary))
  (bind _output_get (Variables|Default|SetMaterial _returnvalue))
  (Rendering|Material|SetMaterial (Variables|Character|GetMesh) 1 _output_get))

(event Game|Damage|EventAnyDamage
  (params (Damage :type Float%20%28single-precision%29) (DamageType :type Damage%20Type%20Object%20Reference) (InstigatedBy :type Controller%20Object%20Reference) (DamageCauser :type Actor%20Object%20Reference))
  (bind _killwait (Variables|Default|GetKillWait))
  (|SetDamage InstigatedBy Damage DamageCauser)
  (Variables|Default|SetStateType "NewEnumerator8")
  (Utilities|FlowControl|Sequence
    (:then_0
      (|IsDead))
    (:then_1
      (if (not (Variables|Default|GetKillWait))
        (|PlayHitMontage)))
    (:then_2
      (|DamageFont))
    (:then_3
      (|PlayHitSound))
    (:then_4
      (|PlayHitEffect))
    (:then_5
      (|HitStop (Math|Float|SelectFloat 0.5 0.05 _killwait) (Math|Float|SelectFloat 0.2 0.001 _killwait)))))

(event Custom|KillEvent
  (CallFunction|Killed)
  (Actor|DestroyActor))

(event Custom|RecoverTimeDilation
  (Utilities|Time|SetGlobalTimeDilation 1.0))

(fn GetCanMove
  (return (Variables|Default|GetCanMove)))

(fn GetCombat
  (return (Variables|Default|GetCombatType)))

(fn GetCurrentWeapon
  (return 0))

(fn GetHealth
  (return (Variables|/Game/Components/Status/StatusComponent.StatusComponent_C|GetHealth (Variables|Default|GetStatus))))

(fn GetState
  (return (Variables|Default|GetStateType)))

(fn IsAlive
  (return (Utilities|Enum|NotEqual(Enum) (Variables|Default|GetStateType) "NewEnumerator9")))

(fn SetCanMove
  (params (CanMove :type Boolean))
  (bind _output_get (Variables|Default|SetCanMove CanMove))
  (if _output_get
    _
    (else
      (Components|Movement|StopMovementImmediately (Variables|Character|GetCharacterMovement))))
  (return _output_get))

(fn SetCombat
  (params (CombatType :type ECombatType%20Enum :default "NewEnumerator0"))
  (bind _output_get (Variables|Default|SetCombatType CombatType))
  (return _output_get))

(fn SetHealth
  (params (Health :type Float%20%28single-precision%29))
  (bind _output_get (Variables|/Game/Components/Status/StatusComponent.StatusComponent_C|SetHealth (Variables|Default|GetStatus) Health))
  (return _output_get))

(fn SetState
  (params (StateType :type EStateType%20Enum :default "NewEnumerator0"))
  (bind _output_get (Variables|Default|SetStateType StateType))
  (return _output_get))

(fn WeaponChange
  (params (New%20Weapon :type BP%20Weapon%20Object%20Reference)))

(fn WeaponEquipped
  (params (Combat :type ECombatType%20Enum :default "NewEnumerator0"))
  (Variables|Default|SetStateType "NewEnumerator0")
  (return false))

(fn WeaponGrab
  (params (Combat :type ECombatType%20Enum :default "NewEnumerator0"))
  (return false))

(fn WeaponHitted
  (Variables|Default|SetStateType "NewEnumerator0")
  (return false))

(fn WeaponPlayDrawMontage
  (return false))

(fn WeaponPlayMeleeMontage
  (params (CombatType :type ECombatType%20Enum :default "NewEnumerator0") (MeleeCount :type Integer))
  (bind _meleemontages (Variables|UserSettings|GetMeleeMontages))
  (bind (_value _returnvalue) (Utilities|Map|Find _meleemontages CombatType))
  (bind (_montage _playratio _startsection _canmove) (Utilities|Struct|BreakFMontageData _value))
  (if _returnvalue
    (Animation|PlayAnimMontage _montage _playratio _startsection)
    (CallFunction|SetCanMove _canmove)
    (return true)
    (else
      (return false))))

(fn WeaponPlaySheathMontage
  (return false))

(fn WeaponPlaySkillMontage
  (params (CombatType :type ECombatType%20Enum :default "NewEnumerator0"))
  (return false))

(fn WeaponSheathed
  (Variables|Default|SetStateType "NewEnumerator0")
  (return false))

(fn WeaponUngrab
  (params (Combat :type ECombatType%20Enum :default "NewEnumerator0"))
  (return false))