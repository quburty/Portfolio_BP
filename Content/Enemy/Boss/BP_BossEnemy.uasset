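; Boss enemy Blueprint that adds a fist weapon and two skills, a knockback roar and zombie summoning, to its parent class.
; On BeginPlay it spawns an enlarged fist weapon, attaches it to a hand socket and raises the boss's position.
; SkillRoaring uses a temporary sphere to launch overlapping Characters outward and upward.
; RandomSpawnZombies spawns SpawnNum zombies at random navigable points around the boss; neither skill is called within this Blueprint.
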(event EventBeginPlay
  (|CallParentFunction)
  (bind _returnvalue (Game|SpawnActorfromClass "/Game/Weapons/Melees/BP_Melee_Fist_Boss.BP_Melee_Fist_Boss_C" (Math|Transform|MakeTransform "0, 0, 0" "0, 0, 0" "3.000000,3.000000,3.000000") "Undefined" self 0))
  (bind _output_get (Variables|Default|SetWeapon _returnvalue))
  (Transformation|AttachComponentToComponent _output_get (Variables|Character|GetMesh) "Hand_SubWeapon" "KeepRelative" "KeepRelative" "KeepRelative" true)
  (Transformation|SetActorLocation (+ (Transformation|GetActorLocation) "0, 0,300.000000") false false))

(fn ConstructionScript
  (|CallParentFunction))

(fn SkillRoaring
  (bind _returnvalue (AddComponent|AddSphereComponent false))
  (LocalVariables|SetSphereCollision _returnvalue)
  (Components|Sphere|SetSphereRadius (LocalVariables|GetSphereCollision) 5e+02 true)
  (for _array_element (Collision|GetOverlappingActors (LocalVariables|GetSphereCollision) 0 :!class /Script/Engine.PrimitiveComponent)
    (bind _ascharacter (Utilities|Casting|CastToCharacter _array_element))
    (Physics|AddImpulse (Variables|/Script/Engine.Character|GetCharacterMovement _ascharacter) (Math|Vector|MakeVector (.x (* (Class|KismetMathLibrary|VectorNormal2D (- (Transformation|GetActorLocation _ascharacter) (Transformation|GetActorLocation)) 0.0001) 7.5e+02)) (.y (* (Class|KismetMathLibrary|VectorNormal2D (- (Transformation|GetActorLocation _ascharacter) (Transformation|GetActorLocation)) 0.0001) 7.5e+02)) 3e+02) true))
  (Components|DestroyComponent (LocalVariables|GetSphereCollision)))

(fn RandomSpawnZombies
  (bind _returnvalue (Transformation|GetActorLocation))
  (bind (_randomlocation _returnvalue_2) (Class|NavigationSystemV1|GetRandomPointinNavigableRadius _returnvalue 2e+03 0 0))
  (for _index (range 1 (Variables|Default|GetSpawnNum))
    (if _returnvalue_2
      (Game|SpawnActorfromClass "/Game/Enemy/Zombie/BP_AI_Zombie.BP_AI_Zombie_C" (Math|Transform|MakeTransform (Math|Vector|MakeVector (.x _randomlocation) (.y _randomlocation) (+ (.z _randomlocation) 9e+01))) "AdjustIfPossibleButDontSpawnIfColliding" 0 0))))