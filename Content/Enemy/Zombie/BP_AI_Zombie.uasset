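; Zombie enemy character that fights with a melee fist weapon, built on a parent class.
; On BeginPlay it spawns the enemy fist weapon with itself as owner and attaches it to the mesh's Hand_Weapon socket.
; Weapon_PlayMeleeMontage looks up the combat type in MeleeMontages, plays that montage, applies its movement permission and reports whether an entry was found.
; The melee count input is unused.
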(event EventBeginPlay
  (|CallParentFunction)
  (bind _returnvalue (Game|SpawnActorfromClass "/Game/Weapons/Melees/BP_Melee_Fist_Enemy.BP_Melee_Fist_Enemy_C" (Math|Transform|MakeTransform "0, 0, 0") "Undefined" self 0))
  (bind _output_get (Variables|Default|SetWeapon _returnvalue))
  (Transformation|AttachComponentToComponent _output_get (Variables|Character|GetMesh) "Hand_Weapon" "KeepRelative" "KeepRelative" "KeepRelative" true))

(fn ConstructionScript
  (|CallParentFunction))

(fn WeaponPlayMeleeMontage
  (params (CombatType :type ECombatType%20Enum :default "NewEnumerator0") (MeleeCount :type Integer))
  (bind _meleemontages (Variables|Default|GetMeleeMontages))
  (bind (_value _returnvalue) (Utilities|Map|Find _meleemontages (Variables|Default|GetCombatType)))
  (bind (_montage _playratio _startsection _canmove) (Utilities|Struct|BreakFMontageData _value))
  (if _returnvalue
    (Animation|PlayAnimMontage _montage _playratio _startsection)
    (CallFunction|SetCanMove _canmove)
    (return true)
    (else
      (return false))))